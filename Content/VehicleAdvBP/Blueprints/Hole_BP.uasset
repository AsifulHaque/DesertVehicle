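; Pothole hazard Blueprint that crashes the player's vehicle when it crosses the hole too slowly.
; When the box overlap begins, it compares the player vehicle's displayed speed to a required threshold.
; At sufficient speed, a hidden plane blocks the Vehicle channel to bridge the hole; otherwise it flags the vehicle crashed and fires its crash event once.
; Ending the overlap makes the plane ignore vehicles again and resets the once gate.
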(event `self.ReceiveBeginPlay`
  ;[1 1 1] Put this plane, and box collision inside of each pothole. Resize it to cover the top of the hole only, as the event will happen once the player overlaps the box collision
  (`SceneComponent.SetVisibility` (`self.Plane`) false false))

(event `self.Box.OnComponentBeginOverlap`
  (params (OverlappedComponent :type "PrimitiveComponent Object Reference") (OtherActor :type "Actor Object Reference") (OtherComp :type "PrimitiveComponent Object Reference") (OtherBodyIndex :type Integer) (bFromSweep :type Boolean) (SweepResult :type "HitResult Structure (by ref)"))
  (bind _vehicle_ref (`self.Vehicle_Ref`))
  ;[1 1 1] Put this plane, and box collision inside of each pothole. Resize it to cover the top of the hole only, as the event will happen once the player overlaps the box collision
  (bind _asvehicle_blueprint (cast `/Game/VehicleAdvBP/Blueprints/VehicleBlueprint` (`GameplayStatics.GetPlayerPawn` 0)))
  (bind _output_get (set `self.Vehicle_Ref` _asvehicle_blueprint))
  (if (>= (`KismetStringLibrary.Conv_StringToInt` (`/Game/VehicleAdvBP/Blueprints/VehicleBlueprint.Speed Display String` _output_get)) (`self.Speed Required to not Crash`))
    (`PrimitiveComponent.SetCollisionResponseToChannel` (`self.Plane`) "ECC_Vehicle" "ECR_Block")
    (`KismetSystemLibrary.PrintString` "Speed is high enough" false)
    (else
      (`KismetSystemLibrary.PrintString` "Speed is not high enough" false)
      (set `/Game/VehicleAdvBP/Blueprints/VehicleBlueprint.bCrashed` true _vehicle_ref)
      (`/Engine/EditorBlueprintResources/StandardMacros.DoOnce` false :!label _label
        (:`Completed`
          (`/Game/VehicleAdvBP/Blueprints/VehicleBlueprint.Crash Custom Event` _vehicle_ref))))))

(event `self.Box.OnComponentEndOverlap`
  (params (OverlappedComponent :type "PrimitiveComponent Object Reference") (OtherActor :type "Actor Object Reference") (OtherComp :type "PrimitiveComponent Object Reference") (OtherBodyIndex :type Integer))
  ;[1 1 1] Put this plane, and box collision inside of each pothole. Resize it to cover the top of the hole only, as the event will happen once the player overlaps the box collision
  (`PrimitiveComponent.SetCollisionResponseToChannel` (`self.Plane`) "ECC_Vehicle" "ECR_Ignore")
  (goto _label :!via `Reset`))

(fn `UserConstructionScript`)