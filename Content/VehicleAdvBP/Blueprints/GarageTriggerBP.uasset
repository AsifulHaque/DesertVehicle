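; Garage trigger volume that lets the player's vehicle open upgrades while inside it and can complete a mission.
; Overlap begin and end toggle CanOpenUpgrade on the overlapping VehicleBlueprint.
; On entry at objective index 2, it shows a MISSION COMPLETE HUD warning through VehicleAdvGameMode, stops the timer, advances the objective and halts the vehicle.
; A short delay then hides the warning.
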(event `self.ReceiveActorBeginOverlap`
  (params (OtherActor :type "Actor Object Reference"))
  (bind _asvehicle_blueprint (cast `/Game/VehicleAdvBP/Blueprints/VehicleBlueprint` OtherActor))
  (set `/Game/VehicleAdvBP/Blueprints/VehicleBlueprint.CanOpenUpgrade` true _asvehicle_blueprint)
  (bind _asvehicle_adv_game_mode (cast `/Game/VehicleAdvBP/Blueprints/VehicleAdvGameMode` (`GameplayStatics.GetGameMode`)))
  (if (== (`/Game/VehicleAdvBP/Blueprints/VehicleAdvGameMode.CurrentObjIndex` _asvehicle_adv_game_mode) 2)
    ;[1 1 1] MISSION COMPLETE
    (`/Game/VehicleAdvBP/Blueprints/VehicleAdvGameMode.HUDWarning` _asvehicle_adv_game_mode "MISSION COMPLETE" true false)
    (`/Game/VehicleAdvBP/Blueprints/VehicleAdvGameMode.StopTimer` _asvehicle_adv_game_mode)
    (set `/Game/VehicleAdvBP/Blueprints/VehicleAdvGameMode.CurrentObjIndex` 3 _asvehicle_adv_game_mode)
    (`MovementComponent.StopMovementImmediately` (`WheeledVehicle.VehicleMovement` _asvehicle_blueprint))
    (`KismetSystemLibrary.Delay` 5.0)
    (`/Game/VehicleAdvBP/Blueprints/VehicleAdvGameMode.HUDWarning` _asvehicle_adv_game_mode "MISSION COMPLETE" false false)))

(event `self.ReceiveActorEndOverlap`
  (params (OtherActor :type "Actor Object Reference"))
  (bind _asvehicle_blueprint (cast `/Game/VehicleAdvBP/Blueprints/VehicleBlueprint` OtherActor))
  (set `/Game/VehicleAdvBP/Blueprints/VehicleBlueprint.CanOpenUpgrade` false _asvehicle_blueprint))

(fn `UserConstructionScript`)