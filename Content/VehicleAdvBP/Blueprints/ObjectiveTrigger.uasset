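; Objective trigger actor for the flag goal, fired when the player's VehicleBlueprint overlaps it while the game mode's objective index is not already 2.
; It saves the vehicle's location and rotation as its respawn point and sets the objective index to 2 on the cached VehicleAdvGameMode.
; It shows a timed "reached the flag" HUD message and makes the referenced trophy's mesh visible as the badge to collect at the ship.
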(event `self.ReceiveBeginPlay`
  ;[1 1 1] Set a ref to GM
  (bind _asvehicle_adv_game_mode (cast `/Game/VehicleAdvBP/Blueprints/VehicleAdvGameMode` (`GameplayStatics.GetGameMode`)))
  (set `self.GameModeref` _asvehicle_adv_game_mode))

(event `self.ReceiveActorBeginOverlap`
  (params (OtherActor :type "Actor Object Reference"))
  (bind _gamemoderef (`self.GameModeref`))
  (bind _tropy (`self.Tropy`))
  (bind _asvehicle_blueprint (cast `/Game/VehicleAdvBP/Blueprints/VehicleBlueprint` OtherActor))
  (if (not (== (`/Game/VehicleAdvBP/Blueprints/VehicleAdvGameMode.CurrentObjIndex` _gamemoderef) 2))
    ;[1 1 1] SaveLocation for respawning
    (set `/Game/VehicleAdvBP/Blueprints/VehicleBlueprint.StartingRotation` (`self.K2_GetActorRotation` _asvehicle_blueprint) _asvehicle_blueprint)
    (set `/Game/VehicleAdvBP/Blueprints/VehicleBlueprint.StartingLocation` (`self.K2_GetActorLocation` _asvehicle_blueprint) _asvehicle_blueprint)
    (`/Game/VehicleAdvBP/Blueprints/VehicleAdvGameMode.HUDWarning` _gamemoderef "REACHED THE FLAG!!!" true false)
    (set `/Game/VehicleAdvBP/Blueprints/VehicleAdvGameMode.CurrentObjIndex` 2 _gamemoderef)
    (`|ExecutionSequence`
      (:`then_0`
        (`KismetSystemLibrary.Delay` 3.0)
        (`/Game/VehicleAdvBP/Blueprints/VehicleAdvGameMode.HUDWarning` _gamemoderef "REACHED THE FLAG!!!" false false))
      (:`then_1`
        ;[1 1 1] Sets Up Badge to collect at the ship
        (`/Engine/EditorBlueprintResources/StandardMacros.IsValid` _tropy
          (:`Is Valid`
            (`SceneComponent.SetVisibility` (`self.GetComponentByClass` _tropy "/Script/Engine.StaticMeshComponent") true false)))))))

(fn `UserConstructionScript`)