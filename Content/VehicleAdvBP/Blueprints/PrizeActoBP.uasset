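; PrizeActoBP is a collectible badge pickup for the vehicle game that spins its static mesh while visible.
; When a VehicleBlueprint overlaps it, a DoOnce hides the mesh and has VehicleAdvGameMode show a "BADGE EARNED" HUD message.
; After a short delay it clears the message and destroys itself; no badge state is stored here.
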(event `self.ReceiveTick`
  (params (DeltaSeconds :type "Float (single-precision)"))
  (bind _staticmesh (`self.StaticMesh`))
  (if (`SceneComponent.IsVisible` _staticmesh)
    (`SceneComponent.K2_AddRelativeRotation` _staticmesh (struct :`Yaw` 1.5) false false)))

(event `self.ReceiveActorBeginOverlap`
  (params (OtherActor :type "Actor Object Reference"))
  (cast `/Game/VehicleAdvBP/Blueprints/VehicleBlueprint` OtherActor)
  (if (`SceneComponent.IsVisible` (`self.StaticMesh`))
    (`/Engine/EditorBlueprintResources/StandardMacros.DoOnce` false
      (:`Completed`
        (`SceneComponent.SetVisibility` (`self.StaticMesh`) false false)
        (bind _asvehicle_adv_game_mode (cast `/Game/VehicleAdvBP/Blueprints/VehicleAdvGameMode` (`GameplayStatics.GetGameMode`)))
        (`/Game/VehicleAdvBP/Blueprints/VehicleAdvGameMode.HUDWarning` _asvehicle_adv_game_mode "BADGE EARNED" true false)
        (`KismetSystemLibrary.Delay` 3.0)
        (`/Game/VehicleAdvBP/Blueprints/VehicleAdvGameMode.HUDWarning` _asvehicle_adv_game_mode "BADGE EARNED" false false)
        (`self.K2_DestroyActor`)))))

(fn `UserConstructionScript`)